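; AR debugging component on BP_ARController that visualizes tracking state and can start debug or release AR sessions.
; Each tick it labels planes, diffs tracked images and, on AR devices, updates tracking info, pushing changes through server calls.
; Poses are stored pawn-relative, then rebuilt in world space to draw toggleable camera, pawn, origin and image gizmos.
; Image boxes show tracking state and relocalizer picks; non-AR devices add camera-distance lines.
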(event `self.ReceiveBeginPlay`
  (`self.Initialize`))

(event `self.OnNotify_PlaneRendererSpawned`
  (bind _planerenderer (`self.PlaneRenderer`))
  (if (`KismetSystemLibrary.IsValid` _planerenderer)
    (`DDBlueprintLibrary.LogDebug` "Initializing PlaneRenderer")
    (set `ARPlaneRenderer.PlaneMaterial` "/DDAugmented/Assets/Materials/ARPlane_Mat.ARPlane_Mat" _planerenderer)
    (set `ARPlaneRenderer.PlaneColors` (`self.planeColors`) _planerenderer)
    (else
      (`DDBlueprintLibrary.LogError` "Can't initialize PlaneRenderer -- it's NULL"))))

(event `self.ReceiveTick`
  (params (DeltaSeconds :type "Float (single-precision)"))
  (`|ExecutionSequence`
    (:`then_0`
      (bind _returnvalue (`ARBlueprintLibrary.GetAllTrackedPlanes`))
      (for _array_element _returnvalue
        (`KismetSystemLibrary.DrawDebugString` (.location (`ARTrackedGeometry.GetLocalToWorldTransform` _array_element)) (`KismetStringLibrary.Conv_NameToString` (`ARTrackedGeometry.GetDebugName` _array_element)) null)))
    (:`then_1`
      (bind _returnvalue_2 (`ARBlueprintLibrary.GetAllTrackedImages`))
      (`self.Process Tracked Images` _returnvalue_2))
    (:`then_2`
      (bind _returnvalue_3 (`blueprintHelpers.isArCapableDevice`))
      (if _returnvalue_3
        (`self.Update Tracking Info`))
      (`self.Draw Debuggables`))))

(fn `Add Image Tracking Data`
  (params (arImage :type "ARTrackedGeometry Object Reference (by ref)"))
  (returns (imageId :type String))
  (locals (trackedImageData :type "TrackedImageData Structure"))
  (bind _asartracked_image (cast `ARTrackedImage` arImage))
  (bind _output_get (set `local.trackedImageData` (`self.Make Image Tracking Info` _asartracked_image)))
  (`KismetArrayLibrary.Array_Add` (`self.TrackedImages`) _output_get)
  (`self.ServerAddTrackedImage` _output_get)
  (return (`KismetGuidLibrary.Conv_GuidToString` (`.id_` (break `TrackedImageData` _output_get)))))

(fn `Draw AR Image`
  (params (imageTrackingData :type "TrackedImageData Structure (by ref)") (fanchor :type "FAnchor Object Reference") (relocalizer :type "/FiducialRelocalizer/BP_Relocalizer Object Reference"))
  (locals (alignedTransform :type "Transform Structure"))
  (bind (_pawntoimage _estimatedsize _trackingstate _imagename _id_ _pickedforestimation) (break `TrackedImageData` imageTrackingData))
  (bind _returnvalue (`KismetMathLibrary.ComposeTransforms` _pawntoimage (`self.Get Pawn World T`)))
  (bind (_x _y) (`KismetMathLibrary.BreakVector2D` _estimatedsize))
  (bind _location (.location (`self.Get Camera World T`)))
  (bind _location_2 (.location _returnvalue))
  (bind _returnvalue_2 (/ (`KismetMathLibrary.MakeVector` _y _x) 2.0))
  (set `local.alignedTransform` _returnvalue)
  (`self.Draw Pose` _returnvalue _imagename)
  (`KismetSystemLibrary.DrawDebugBox` _location_2 _returnvalue_2 (select `EARTrackingState` _trackingstate :`Unknown` (struct :`R` 0.955151 :`G` 1.0 :`B` 0.98169 :`A` 1.0) :`Tracking` (struct :`G` 1.0 :`B` 0.092009 :`A` 1.0) :`NotTracking` (struct :`R` 1.0 :`A` 1.0) :`StoppedTracking` (struct :`R` 1.0 :`G` 0.930819 :`A` 1.0) :!type "LinearColor Structure") (.rotation _returnvalue) 0.0 0.5)
  (if _pickedforestimation
    (`KismetSystemLibrary.DrawDebugBox` (.location (`local.alignedTransform`)) (* _returnvalue_2 1.1) (struct :`R` 0.617258 :`B` 0.759827 :`A` 1.0) (.rotation (`local.alignedTransform`)) 0.0 1.0))
  (bind _returnvalue_3 (`blueprintHelpers.isArCapableDevice`))
  (if (not _returnvalue_3)
    (`KismetSystemLibrary.DrawDebugLine` _location _location_2 (struct :`R` 0.949443 :`G` 0.842717 :`A` 1.0) 0.0 0.5)
    (`KismetSystemLibrary.DrawDebugString` (/ (+ _location _location_2) 2.0) (`KismetStringLibrary.Conv_DoubleToString` (`KismetMathLibrary.VSize` (- _location _location_2))) null)))

(fn `Draw AR Images`
  (locals (fiducialRelocalizer :type "/FiducialRelocalizer/BP_Relocalizer Object Reference"))
  (bind _fiducialrelocalizer (`local.fiducialRelocalizer`))
  (set `local.fiducialRelocalizer` (`Actor.GetComponentByClass` (`GameplayStatics.GetPlayerController` 0) "/FiducialRelocalizer/BP_Relocalizer.BP_Relocalizer_C"))
  (for _array_element (`self.TrackedImages`)
    (`self.Draw AR Image` _array_element (`ARTrackedFiducial.getFiducialAnchor` (`BlueprintMapLibrary.Map_Find` (`FiducialRelocalizerComponent.GetActiveFiducials` _fiducialrelocalizer) (`.ImageName` (break `TrackedImageData` _array_element)))) _fiducialrelocalizer)))

(fn `Draw Debuggables`
  (locals (pawn :type "/Game/Blueprints/BP_ARPawn Object Reference"))
  (bind _pawn (`local.pawn`))
  (bind _returnvalue (`SceneComponent.K2_GetComponentToWorld` (`/Game/Blueprints/BP_ARPawn.DefaultSceneRoot` _pawn)))
  (bind _pawn_2 (`self.Get Pawn`))
  (set `local.pawn` _pawn_2)
  (if (`self.Has Pawn`)
    (`|ExecutionSequence`
      (:`then_0`
        (if (`self.isRenderingCamera`)
          (`self.Draw Pose` (`KismetMathLibrary.ComposeTransforms` (`/Game/Blueprints/BP_ARPawn.cameraTransform` _pawn) _returnvalue) "AR CAMERA" 3.0)))
      (:`then_1`
        (if (`self.isRenderingPawn`)
          (`self.Draw Pose` _returnvalue "AR PAWN" 2.0)))
      (:`then_2`
        (if (`self.isRenderingTrackOrigin`)
          (`self.Draw Pose` (`KismetMathLibrary.ComposeTransforms` (`.PawnToTrackOrigin` (break `TrackingInfo` (`self.TrackingInfo`))) _returnvalue) "TRACK ORIGIN" 2.0)))
      (:`then_3`
        (if (`self.isRenderingImages`)
          (`self.Draw AR Images`))))))

(fn `Draw Pose`
  (params (transform :type "Transform Structure (by ref)") (label :type String) (scale :type "Float (double-precision)" :default 1.0))
  (bind _location (.location transform))
  (`KismetSystemLibrary.DrawDebugString` _location (`KismetTextLibrary.Conv_TextToString` (`|FormatText` "{label}\n{transform}\n{rotator}" (`KismetTextLibrary.Conv_StringToText` label) (`KismetTextLibrary.Conv_VectorToText` _location) (`KismetTextLibrary.Conv_RotatorToText` (.rotation transform)))) null (struct :`R` 1.0 :`G` 0.04564 :`B` 0.036081 :`A` 1.0))
  (`KismetSystemLibrary.DrawDebugArrow` _location (.location (`KismetMathLibrary.ComposeTransforms` (`self.Scaled X Axis` scale) transform)) 0.5 (struct :`R` 1.0 :`G` 0.01504 :`A` 1.0) 0.0 0.5)
  (`KismetSystemLibrary.DrawDebugArrow` _location (.location (`KismetMathLibrary.ComposeTransforms` (`self.Scaled Y Axis` scale) transform)) 0.5 (struct :`R` 0.135686 :`G` 1.0 :`A` 1.0) 0.0 0.5)
  (`KismetSystemLibrary.DrawDebugArrow` _location (.location (`KismetMathLibrary.ComposeTransforms` (`self.Scaled Z Axis` scale) transform)) 0.5 (struct :`G` 0.286275 :`B` 1.0 :`A` 1.0) 0.0 0.5))

(fn `Get AR Alignment T`
  (returns (t :type "Transform Structure"))
  (return (`.TrackingAlignment` (break `TrackingInfo` (`self.TrackingInfo`)))))

(fn `Get Camera Relative T`
  (returns (t :type "Transform Structure"))
  (bind _pawn (`self.Get Pawn`))
  (return (`SceneComponent.GetRelativeTransform` (`/Game/Blueprints/BP_ARPawn.Camera` _pawn))))

(fn `Get Camera Tracking T`
  (returns (t :type "Transform Structure"))
  (return (`KismetMathLibrary.ComposeTransforms` (`self.Get Camera Relative T`) (`self.Get Pawn Tracking T`))))

(fn `Get Camera World T`
  (returns (t :type "Transform Structure"))
  (bind _pawn (`self.Get Pawn`))
  (return (`SceneComponent.K2_GetComponentToWorld` (`/Game/Blueprints/BP_ARPawn.Camera` _pawn))))

(fn `Get Controller`
  (returns (controller :type "/Game/Blueprints/BP_ARController Object Reference"))
  (if (not (`KismetSystemLibrary.IsValid` (`self.ArController`)))
    (bind _asbp_arcontroller (cast `/Game/Blueprints/BP_ARController` (`self.GetOwner`))
      (:`then`
        (set `self.ArController` _asbp_arcontroller))
      (:`CastFailed`
        _)))
  (bind _asbp_arcontroller_2 (cast `/Game/Blueprints/BP_ARController` (`self.ArController`))
    (:`then`
      (return _asbp_arcontroller_2))
    (:`CastFailed`
      (return null))))

(fn `Get Pawn`
  (returns (pawn :type "/Game/Blueprints/BP_ARPawn Object Reference"))
  (if (not (`KismetSystemLibrary.IsValid` (`self.ArPawn`)))
    (bind _controller (`self.Get Controller`))
    (if (`KismetSystemLibrary.IsValid` _controller)
      (set `self.ArPawn` (`Controller.K2_GetPawn` _controller))))
  (bind _asbp_arpawn (cast `/Game/Blueprints/BP_ARPawn` (`self.ArPawn`))
    (:`then`
      (return _asbp_arpawn))
    (:`CastFailed`
      (return null))))

(fn `Get Pawn Tracking T`
  (returns (t :type "Transform Structure"))
  (if (`KismetSystemLibrary.IsValid` (`self.ArPawn`))
    (return (`KismetMathLibrary.InvertTransform` (`.PawnToTrackOrigin` (break `TrackingInfo` (`self.TrackingInfo`)))))
    (else
      (return (`KismetMathLibrary.MakeTransform` (0.0 0.0 0.0))))))

(fn `Get Pawn World T`
  (returns (t :type "Transform Structure"))
  (bind _pawn (`self.Get Pawn`))
  (if (`KismetSystemLibrary.IsValid` _pawn)
    (return (`Actor.GetTransform` _pawn))
    (else
      (return (`KismetMathLibrary.MakeTransform` (0.0 0.0 0.0))))))

(fn `Has Pawn`
  (returns (hasPawn :type Boolean))
  (return (`KismetSystemLibrary.IsValid` (`self.ArPawn`))))

(fn `Init Debubg Session`
  (`ARBlueprintLibrary.StartARSession` "/DDAugmented/Data/D_DebugSessionConfig.D_DebugSessionConfig")
  (set `self.isDebugSession` true))

(fn `Init Release Session`
  (params (config :type "ARSessionConfig Object Reference"))
  (bind _output_get (set `self.releaseSessionConfig` config))
  (`ARBlueprintLibrary.StartARSession` _output_get)
  (set `self.isDebugSession` false))

(fn `Initialize`
  (`/Engine/EditorBlueprintResources/StandardMacros.IsValid` (`self.releaseSessionConfig`)
    (:`Is Not Valid`
      (switch `EARSessionStatus` (`.Status` (break `ARSessionStatus` (`ARBlueprintLibrary.GetARSessionStatus`)))
        (:`Running`
          (set `self.releaseSessionConfig` (`ARBlueprintLibrary.GetSessionConfig`)))))))

(fn `Make Image Tracking Info`
  (params (arImage :type "ARTrackedImage Object Reference"))
  (returns (TrackedImageData :type "TrackedImageData Structure"))
  (bind _structout (setmembers `TrackedImageData` :`StructRef` (`self.MakeNewTrackedImageData` self) :`PawnToImage` (`KismetMathLibrary.MakeRelativeTransform` (`ARTrackedGeometry.GetLocalToWorldTransform` arImage) (`self.Get Pawn World T`)) :`EstimatedSize` (`ARTrackedImage.GetEstimateSize` arImage) :`TrackingState` (`ARTrackedGeometry.GetTrackingState` arImage) :`ImageName` (`ARCandidateImage.GetFriendlyName` (`ARTrackedImage.GetDetectedImage` arImage)) :`PickedForEstimation` (`/FiducialRelocalizer/BP_Relocalizer.Is Picked For Estimation` (`Actor.GetComponentByClass` (`self.GetOwner`) "/FiducialRelocalizer/BP_Relocalizer.BP_Relocalizer_C") arImage)))
  (return _structout))

(fn `OnRep_trackedImages`)

(fn `Process Tracked Images`
  (params (images :type "Array of ARTrackedGeometry Object Reference (by ref)"))
  (locals (oldTrackedImages :type "Set of ARTrackedGeometry Object Reference") (removeIds :type "Array of String"))
  (bind _arimageidmap (`self.arImageIdMap`))
  (bind _arimageidmap_2 (`self.arImageIdMap`))
  (bind _removeids (`local.removeIds`))
  (bind _returnvalue (`KismetArrayLibrary.Array_Length` _removeids))
  (bind _keys (`BlueprintMapLibrary.Map_Keys` (`self.arImageIdMap`)))
  (`BlueprintSetLibrary.Set_AddItems` (`local.oldTrackedImages`) _keys)
  (for _array_element images
    (if (`KismetArrayLibrary.Array_Contains` _keys _array_element)
      (`BlueprintSetLibrary.Set_Remove` (`local.oldTrackedImages`) _array_element)
      (`self.Update Image Tracking Data` (`BlueprintMapLibrary.Map_Find` _arimageidmap _array_element) _array_element)
      (else
        (bind _imageid (`self.Add Image Tracking Data` _array_element))
        (`BlueprintMapLibrary.Map_Add` _arimageidmap _array_element _imageid))))
  ;[1 1 1] Handle Deletion of Old Images
  (bind _result (`BlueprintSetLibrary.Set_ToArray` (`local.oldTrackedImages`)))
  (for _array_element_2 _result
    (bind _value (`BlueprintMapLibrary.Map_Find` _arimageidmap_2 _array_element_2))
    (`KismetArrayLibrary.Array_Add` (`local.removeIds`) _value)
    (`BlueprintMapLibrary.Map_Remove` _arimageidmap_2 _array_element_2)
    (`self.Remove Image Tracking Data` _value))
  (if (> _returnvalue 0)
    (`DDBlueprintLibrary.LogDebug` (`KismetTextLibrary.Conv_TextToString` (`|FormatText` "Deleting {nImages} old images" _returnvalue)))
    (`self.ServerRemoveTrackedImage` _removeids)))

(fn `Remove Image Tracking Data`
  (params (dataId :type String))
  (bind _trackedimages (`self.TrackedImages`))
  (for _array_element _trackedimages
    (if (`KismetStringLibrary.EqualEqual_StrStr` dataId (`.ImageName` (break `TrackedImageData` _array_element)))
      (`KismetArrayLibrary.Array_RemoveItem` _trackedimages _array_element)
      (break))))

(fn `Send Camera Adjustment`
  (params (adjustmentT :type "Transform Structure (by ref)")))

(fn `Send Pawn Adjustment`
  (params (adjustmentT :type "Transform Structure (by ref)")))

(fn `Update Image Tracking Data`
  (params (trackingId :type String) (arImage :type "ARTrackedGeometry Object Reference"))
  (locals (imageTrackingInfo :type "TrackedImageData Structure") (updatedData :type "Array of TrackedImageData Structure"))
  (bind _trackedimages (`self.TrackedImages`))
  (bind _asartracked_image (cast `ARTrackedImage` arImage))
  (for (_ _array_index) _trackedimages
    (bind _output (`|GetArrayItem` _trackedimages _array_index))
    (if (`KismetStringLibrary.EqualEqual_StrStr` trackingId (`KismetGuidLibrary.Conv_GuidToString` (`.id_` (break `TrackedImageData` _output))))
      (bind (_pawntoimage _estimatedsize _trackingstate _imagename _id_ _pickedforestimation) (break `TrackedImageData` (`self.Make Image Tracking Info` _asartracked_image)))
      (bind _structout (setmembers `TrackedImageData` :`StructRef` _output :`PawnToImage` _pawntoimage :`EstimatedSize` _estimatedsize :`TrackingState` _trackingstate :`PickedForEstimation` _pickedforestimation))
      (`self.ServerUpdateTrackedImage` _structout)
      (break))))

(fn `Update Tracking Info`
  (locals (isTracking :type Boolean))
  (bind (_additionalinfo _status) (break `ARSessionStatus` (`ARBlueprintLibrary.GetARSessionStatus`)))
  (bind _controller (`self.Get Controller`))
  (bind _pawn (`self.Get Pawn`))
  (bind _returnvalue (`HeadMountedDisplayFunctionLibrary.GetTrackingToWorldTransform`))
  (bind _aralignment (`ARBasePlayerController.ArAlignment` _controller))
  (bind _trackinginfo (make `TrackingInfo` (`KismetMathLibrary.MakeRelativeTransform` _aralignment (`KismetMathLibrary.ComposeTransforms` (`SceneComponent.K2_GetComponentToWorld` (`/Game/Blueprints/BP_ARPawn.DefaultSceneRoot` _pawn)) (`KismetMathLibrary.InvertTransform` _returnvalue))) _status _additionalinfo (`ARBlueprintLibrary.GetTrackingQuality`) (`ARBlueprintLibrary.GetWorldMappingStatus`) _aralignment))
  (bind _returnvalue_2 (`self.Equals` self (`self.TrackingInfo`) _trackinginfo))
  (if (not _returnvalue_2)
    (bind _output_get (set `self.TrackingInfo` _trackinginfo))
    (bind _controller_2 (`self.Get Controller`))
    (if (not (`Actor.HasAuthority` _controller_2))
      (`self.ServerUpdateTrackingInfo` self _output_get))))